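; Enemy Blueprint that shows a health bar above the enemy through a world-space widget component.
; Each tick it casts the widget to HealthBar and sets the progress bar from CurrentHealth, assuming a maximum of 100.
; It also rotates the widget every tick to face the first player character's location, billboard style.
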(event EventBeginPlay)

(event Collision|EventActorBeginOverlap
  (params (OtherActor :type Actor%20Object%20Reference)))

(event EventTick
  (params (DeltaSeconds :type Float%20%28single-precision%29))
  (bind _widget (Variables|Default|GetWidget))
  (bind _ashealth_bar (Utilities|Casting|CastToHealthBar (UserInterface|GetUserWidgetObject (Variables|Default|GetWidget))))
  (Progress|SetPercent (Variables|/Game/Widgets/HealthBar.HealthBar_C|GetProgressBar_64 _ashealth_bar) (/ (Variables|Default|GetcurrentHealth) 1e+02))
  (Transformation|SetWorldRotation _widget (Math|Rotator|FindLookatRotation (Transformation|GetWorldLocation _widget) (Transformation|GetActorLocation (Game|GetPlayerCharacter 0))) false false))

(fn ConstructionScript)